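; BP_Weapon is a weapon pickup that a character equips by interacting with it.
; Its Interaction event snaps the weapon onto the WEAPONDERECHA socket of the interacting character's mesh.
; It then turns off collision on RadioInteract and messages the character to remove it as an interactable object.
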(event EventBeginPlay
  (|CallParentFunction) ; This node is disabled and will not be called.\nDrag off pins to build functionality.
)

(event Collision|EventActorBeginOverlap
  (params (OtherActor :type Actor%20Object%20Reference))
  (|CallParentFunction OtherActor) ; This node is disabled and will not be called.\nDrag off pins to build functionality.
)

(event EventTick
  (params (DeltaSeconds :type Float%20%28single-precision%29))
  (|CallParentFunction DeltaSeconds) ; This node is disabled and will not be called.\nDrag off pins to build functionality.
)

(event EventInteraction
  (params (CharRef :type Character%20Object%20Reference))
  (Transformation|AttachComponentToComponent (Variables|/Script/Engine.Character|GetMesh CharRef) "WEAPONDERECHA" "SnapToTarget" "SnapToTarget" "SnapToTarget" true)
  (Collision|SetCollisionEnabled (Variables|Default|GetRadioInteract) "NoCollision")
  (Class|BPLPlayer|RemoveInteractableObj(Message) CharRef self))

(fn ConstructionScript
  (|CallParentFunction))