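; Player Blueprint that lets the player interact with registered items in the game.
; Add and remove events maintain an array of interactable items.
; On the Interact input action's Triggered event, it sends an interaction message to the first item in that array, if any, passing itself.
; BeginPlay, overlap and Tick are unused, and the construction script only calls its parent.
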(event Input|EnhancedActionEvents|EnhancedInputActionIA_Interact
  (params (ActionValue :type Boolean) (ElapsedSeconds :type Float%20%28double-precision%29) (TriggeredSeconds :type Float%20%28double-precision%29) (InputAction :type Input%20Action%20Object%20Reference :default "/Game/Blueprint/IA_Interact.IA_Interact"))
  (:Triggered
    (if (Utilities|Array|IsNotEmpty (Variables|Default|GetInterableItems))
      (Class|InterfaceInteractuable|Interaction(Message) (Utilities|Array|Get(acopy) (Variables|Default|GetInterableItems)) self))))

(event EventBeginPlay)

(event Collision|EventActorBeginOverlap
  (params (OtherActor :type Actor%20Object%20Reference)))

(event EventTick
  (params (DeltaSeconds :type Float%20%28single-precision%29)))

(event EventAddInterectableObj
  (params (Item :type Actor%20Object%20Reference))
  (Utilities|Array|Add (Variables|Default|GetInterableItems) Item))

(event EventRemoveInteractableObj
  (params (Item :type Actor%20Object%20Reference))
  (Utilities|Array|RemoveItem (Variables|Default|GetInterableItems) Item))

(fn ConstructionScript
  (|CallParentFunction))